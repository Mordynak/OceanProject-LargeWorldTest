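; A free-flying, six-degree-of-freedom player pawn that shows a controls widget on screen at BeginPlay.
; Forward, right and lift axes add linear velocity to the physics-driven static mesh along the actor's forward, right and up vectors.
; Look and roll axes apply local pitch, yaw and roll rotation directly to the actor, without frame-time scaling.
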(event EventBeginPlay
  (bind _returnvalue (UserInterface|CreateWidget "/Game/Composition/Blueprints/WB_Controls.WB_Controls_C"))
  (UserInterface|Viewport|AddtoViewport _returnvalue 0))

(event Input|AxisEvents|InputAxisMoveForward
  (params (AxisValue :type Float%20%28single-precision%29))
  (Physics|SetPhysicsLinearVelocity (Variables|Default|GetStaticMesh) (* (Math|Vector|GetForwardVector (Transformation|GetActorRotation)) (* AxisValue 1e+02)) true "None"))

(event Input|AxisEvents|InputAxisMoveRight
  (params (AxisValue :type Float%20%28single-precision%29))
  (Physics|SetPhysicsLinearVelocity (Variables|Default|GetStaticMesh) (* (Math|Vector|GetRightVector (Transformation|GetActorRotation)) (* AxisValue 1e+02)) true "None"))

(event Input|AxisEvents|InputAxisLookUp
  (params (AxisValue :type Float%20%28single-precision%29))
  (Transformation|AddActorLocalRotation (Math|Rotator|MakeRotator 0.0 AxisValue 0.0) false false))

(event Input|AxisEvents|InputAxisLookRight
  (params (AxisValue :type Float%20%28single-precision%29))
  (Transformation|AddActorLocalRotation (Math|Rotator|MakeRotator 0.0 0.0 AxisValue) false false))

(event Input|AxisEvents|InputAxisRoll
  (params (AxisValue :type Float%20%28single-precision%29))
  (Transformation|AddActorLocalRotation (Math|Rotator|MakeRotator AxisValue 0.0 0.0) false false))

(event Input|AxisEvents|InputAxisLift
  (params (AxisValue :type Float%20%28single-precision%29))
  (Physics|SetPhysicsLinearVelocity (Variables|Default|GetStaticMesh) (* (Math|Vector|GetUpVector (Transformation|GetActorRotation)) (* AxisValue 1e+02)) true "None"))

(fn ConstructionScript)